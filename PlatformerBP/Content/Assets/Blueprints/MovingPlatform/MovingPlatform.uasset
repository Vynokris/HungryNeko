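; Moving platform that carries the player along a spline path.
; When a "Player"-tagged actor enters the detector, a timeline plays and moves the box collider to the matching distance along the spline, matching its yaw to the path direction.
; When the player leaves, the timeline reverses, sending the platform back toward the start.
; On BeginPlay the box is yawed to face the start of the path.
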(event OnComponentBeginOverlap(PlayerDetector)
  (params (OverlappedComponent :type Primitive%20Component%20Object%20Reference) (OtherActor :type Actor%20Object%20Reference) (OtherComp :type Primitive%20Component%20Object%20Reference) (OtherBodyIndex :type Integer) (bFromSweep :type Boolean) (SweepResult :type Hit%20Result%20Structure%20%28by%20ref%29))
  (bind _path (Variables|Default|GetPath))
  (bind _boxcollider (Variables|Default|GetBoxCollider))
  ;[1 1 1] Follow the path when the player is on the platform
  (if (Utilities|Array|ContainsItem (Variables|/Script/Engine.Actor|GetTags OtherActor) "Player")
    (bind _traveldistance (Timeline|PlatformMovement Play)
      (:Update
        (Transformation|SetWorldLocation _boxcollider (Spline|GetLocationatDistanceAlongSpline _path (* _traveldistance (Spline|GetSplineLength (Variables|Default|GetPath))) "World") false false)
        (Transformation|SetRelativeRotation _boxcollider (Math|Rotator|MakeRotator 0.0 0.0 (.yaw (Spline|GetRotationatDistanceAlongSpline _path (* _traveldistance (Spline|GetSplineLength (Variables|Default|GetPath))) "Local"))) false false)))))

(event OnComponentEndOverlap(PlayerDetector)
  (params (OverlappedComponent :type Primitive%20Component%20Object%20Reference) (OtherActor :type Actor%20Object%20Reference) (OtherComp :type Primitive%20Component%20Object%20Reference) (OtherBodyIndex :type Integer))
  (bind _path (Variables|Default|GetPath))
  (bind _boxcollider (Variables|Default|GetBoxCollider))
  ;[1 1 1] Follow the path when the player is on the platform
  (if (Utilities|Array|ContainsItem (Variables|/Script/Engine.Actor|GetTags OtherActor) "Player")
    (bind _traveldistance (Timeline|PlatformMovement Reverse)
      (:Update
        (Transformation|SetWorldLocation _boxcollider (Spline|GetLocationatDistanceAlongSpline _path (* _traveldistance (Spline|GetSplineLength (Variables|Default|GetPath))) "World") false false)
        (Transformation|SetRelativeRotation _boxcollider (Math|Rotator|MakeRotator 0.0 0.0 (.yaw (Spline|GetRotationatDistanceAlongSpline _path (* _traveldistance (Spline|GetSplineLength (Variables|Default|GetPath))) "Local"))) false false)))))

(event EventBeginPlay
  ;[1 1 1] Rotate to face the start of the path
  (Transformation|SetRelativeRotation (Variables|Default|GetBoxCollider) (Math|Rotator|MakeRotator 0.0 0.0 (.yaw (Spline|GetRotationatDistanceAlongSpline (Variables|Default|GetPath) 0.0 "Local"))) false false))

(fn ConstructionScript)