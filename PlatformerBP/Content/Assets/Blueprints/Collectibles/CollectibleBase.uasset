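; CollectibleBase is an actor Blueprint that, by its name, serves as the base for collectibles, providing their spin-and-bob idle motion.
; Each Tick adds RotationSpeed as world yaw and offsets the current Z by a cosine of time since creation, shaped by MovementSpeed and MovementAmplitude.
; Both increments ignore delta time, so spin rate and bob height depend on frame rate.
; It contains no pickup logic.
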(event EventTick
  (params (DeltaSeconds :type Float%20%28single-precision%29))
  (bind _returnvalue (Transformation|GetActorLocation))
  (bind (_x _y _z) (Math|Vector|BreakVector _returnvalue))
  ;[1 1 1] Movement
  (Class|Actor|AddActorWorldRotation (Math|Rotator|MakeRotator 0.0 0.0 (Variables|Default|GetrotationSpeed)))
  (Transformation|SetActorLocation (Math|Vector|MakeVector _x _y (+ _z (* (Math|Trig|Cos(Radians) (* (Actor|GetGameTimeSinceCreation) (Variables|Default|GetmovementSpeed))) (Variables|Default|GetmovementAmplitude)))) false false))

(fn ConstructionScript)