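; Player character Blueprint with camera-relative movement, toggle sprint, crouch, double jump, ground slide, wall slide and wall jump, plus health lost on Enemy overlap.
; Tick resets double jump, decays slide speed via crouched max speed and runs a forward trace for vertical walls.
; The stored wall normal constrains movement, slows falls and blocks re-sliding the same surface until landing.
; Jump input triggers all jump types; death only prints a message.
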(event Custom|Death
  ;[1 1 1] Health
  (Development|PrintString "Player is dead!"))

(event Custom|ResetDoubleJump
  ;[1 1 1] Double-Jumping
  ;;[1 1 1] Reset
  (if (and (AI|Components|NavMovement|IsMovingonGround (Variables|Character|GetCharacterMovement)) (Variables|Default|GethasDoubleJumped))
    (Variables|Default|SethasDoubleJumped false)))

(event Custom|WallSlide
  (bind _returnvalue (Transformation|GetActorLocation))
  (bind _charactermovement (Variables|Character|GetCharacterMovement))
  ;[1 1 1] Wall Sliding
  ;;[1 1 1] Reset
  (if (AI|Components|NavMovement|IsMovingonGround (Variables|Character|GetCharacterMovement))
    (if (Class|KismetMathLibrary|NotEqualExactlyVectorVector (Variables|Default|GetwallSlideNormal) "0, 0, 0")
      (Variables|Default|SetwallSlideNormal "0, 0, 0"))
    (elif (< (.Z (Math|Vector|BreakVector (Variables|/Script/Engine.MovementComponent|GetVelocity (Variables|Character|GetCharacterMovement)))) 0.0)
      ;;[1 1 1] Check if the player is against a wall
      (bind (_outhit _returnvalue_2) (Collision|LineTraceByChannel _returnvalue (+ _returnvalue (* (Transformation|GetActorForwardVector) 5e+01)) "TraceTypeQuery1" false 0 "None"))
      (if (Math|Boolean|ANDBoolean _returnvalue_2 (or (Variables|Default|GetisWallSliding) (Math|Vector|NotEqual(Vector) (Variables|Default|GetwallSlideNormal) (.ImpactNormal (Collision|BreakHitResult _outhit)) 0.0001)) (<= (Math|Vector|DotProduct (.ImpactNormal (Collision|BreakHitResult _outhit)) "0,0.000000,1.000000") 0.1))
        (Variables|Default|SetisWallSliding true)
        (Variables|Default|SetwallSlideNormal (.ImpactNormal (Collision|BreakHitResult _outhit)))
        (Transformation|SetActorRotation (Math|Conversions|RotationFromXVector (* (.ImpactNormal (Collision|BreakHitResult _outhit)) -1.0)))
        ;;[1 1 1] Slow down the fall
        (Variables|/Script/Engine.MovementComponent|SetVelocity _charactermovement (Math|Vector|MakeVector (.X (Math|Vector|BreakVector (* (Variables|Default|GetwallSlideNormal) (Math|Vector|DotProduct (Variables|/Script/Engine.MovementComponent|GetVelocity _charactermovement) (Variables|Default|GetwallSlideNormal))))) (.Y (Math|Vector|BreakVector (* (Variables|Default|GetwallSlideNormal) (Math|Vector|DotProduct (Variables|/Script/Engine.MovementComponent|GetVelocity _charactermovement) (Variables|Default|GetwallSlideNormal))))) (* -1 (Variables|Default|GetwallSlideSpeed))))
        (else
          (Variables|Default|SetisWallSliding false)))
      (elif (Variables|Default|GetisWallSliding)
        (Variables|Default|SetisWallSliding false)))))

(event Custom|DoubleJump
  ;[1 1 1] Double-Jumping
  (if (Math|Boolean|ANDBoolean (AI|Components|NavMovement|IsFalling (Variables|Character|GetCharacterMovement)) (not (Variables|Default|GethasDoubleJumped)) (not (Variables|Default|GetisWallSliding)))
    (Character|LaunchCharacter (Math|Vector|MakeVector 0.0 0.0 (+ (* (.Z (Math|Vector|BreakVector (Variables|/Script/Engine.MovementComponent|GetVelocity (Variables|Character|GetCharacterMovement)))) -1.0) (Variables|Default|GetdoubleJumpZVelocity))) false false)
    (Variables|Default|SethasDoubleJumped true)))

(event Custom|WallJump
  ;[1 1 1] Wall Jump
  (if (Variables|Default|GetisWallSliding)
    (Character|LaunchCharacter (+ (* (* (Math|Vector|GetForwardVector (Transformation|GetActorRotation)) (Variables|Default|GetwallJumpXYVelocity)) -1.0) (Math|Vector|MakeVector 0.0 0.0 (Variables|Default|GetwallJumpZVelocity))) false false)
    (Transformation|SetActorRotation (Math|Conversions|RotationFromXVector (Variables|Default|GetwallSlideNormal)))
    (Variables|Default|SetisWallSliding false)))

(event Custom|MoveInDirection
  (params (Direction :type Vector) (Scale%20Value :type Float%20%28single-precision%29))
  (bind _wallslidenormal (Variables|Default|GetwallSlideNormal))
  ;[1 1 1] Movement
  (if (Variables|Default|GetisWallSliding)
    (Pawn|Input|AddMovementInput _wallslidenormal (* (Math|Vector|DotProduct _wallslidenormal Direction) Scale%20Value) false)
    (else
      (Pawn|Input|AddMovementInput Direction Scale%20Value false))))

(event Custom|GroundSlide
  (bind _charactermovement (Variables|Character|GetCharacterMovement))
  ;[1 1 1] Ground Sliging
  (if (and (Variables|Default|GetisCrouching) (Variables|Default|GetisSprinting))
    (if (> (Variables|/Script/Engine.CharacterMovementComponent|GetMaxWalkSpeedCrouched (Variables|Character|GetCharacterMovement)) (Variables|Default|GetcrouchSpeed))
      (Variables|/Script/Engine.CharacterMovementComponent|SetMaxWalkSpeedCrouched _charactermovement (* (Variables|/Script/Engine.CharacterMovementComponent|GetMaxWalkSpeedCrouched _charactermovement) (Variables|Default|GetgroundSlideFriction) 0.01))
      (else
        (CallFunction|ToggleSprint)))))

(event Custom|ToggleSprint
  ;[1 1 1] Sprinting
  (Utilities|FlowControl|FlipFlop
    (:A
      (Variables|Default|SetisSprinting true)
      (Variables|/Script/Engine.CharacterMovementComponent|SetMaxWalkSpeed (Variables|Character|GetCharacterMovement) (Variables|Default|GetsprintSpeed)))
    (:B
      (Variables|Default|SetisSprinting false)
      (Variables|/Script/Engine.CharacterMovementComponent|SetMaxWalkSpeed (Variables|Character|GetCharacterMovement) (Variables|Default|GetwalkSpeed)))))

(event Collision|EventActorBeginOverlap
  (params (OtherActor :type Actor%20Object%20Reference))
  ;[1 1 1] Health
  (if (Utilities|Array|ContainsItem (Variables|/Script/Engine.Actor|GetTags OtherActor) "Enemy")
    (bind _result (Math|Integer|DecrementInt (Variables|Default|Gethealth))
      (:%20%20
        (if (<= _result 0)
          (CallFunction|Death))))))

(event EventTick
  (params (DeltaSeconds :type Float%20%28single-precision%29))
  ;[1 1 1] Tick Update
  (CallFunction|ResetDoubleJump)
  (CallFunction|WallSlide)
  (CallFunction|GroundSlide))

(event Input|ActionEvents|InputActionJump
  (params (Key :type Key%20Structure :default "None"))
  ;[1 1 1] Jumping
  (:Pressed
    (Character|Jump)
    (CallFunction|DoubleJump)
    (CallFunction|WallJump))
  (:Released
    (Character|StopJumping)))

(event Input|ActionEvents|InputActionSprint
  (params (Key :type Key%20Structure :default "None"))
  ;[1 1 1] Sprinting
  (:Pressed
    (CallFunction|ToggleSprint)))

(event Input|ActionEvents|InputActionCrouch
  (params (Key :type Key%20Structure :default "None"))
  (bind _charactermovement (Variables|Character|GetCharacterMovement))
  ;[1 1 1] Crouching & Ground Slide Start
  (:Pressed
    (if (AI|Components|NavMovement|IsMovingonGround (Variables|Character|GetCharacterMovement))
      (Character|Crouch)
      (Variables|Default|SetisCrouching true)
      (if (Variables|Default|GetisSprinting)
        (Variables|/Script/Engine.CharacterMovementComponent|SetMaxWalkSpeedCrouched _charactermovement (Variables|Default|GetgroundSlideSpeed))
        (bind _forward (CallFunction|GetPawnForward))
        (Pawn|Input|AddMovementInput _forward (Variables|Default|GetgroundSlideSpeed) false)
        (else
          (Variables|/Script/Engine.CharacterMovementComponent|SetMaxWalkSpeedCrouched _charactermovement (Variables|Default|GetcrouchSpeed))))))
  (:Released
    (Character|UnCrouch)
    (Variables|Default|SetisCrouching false)))

(event Input|AxisEvents|InputAxisLateralMovement
  (params (AxisValue :type Float%20%28single-precision%29))
  ;[1 1 1] Movement
  (CallFunction|MoveinDirection (Math|Vector|GetRightVector (Math|Rotator|MakeRotator 0.0 0.0 (.Yaw (Math|Rotator|BreakRotator (Pawn|GetControlRotation :!class /Script/Engine.Pawn))))) AxisValue))

(event Input|AxisEvents|InputAxisForwardMovement
  (params (AxisValue :type Float%20%28single-precision%29))
  ;[1 1 1] Movement
  (CallFunction|MoveinDirection (Math|Vector|GetForwardVector (Math|Rotator|MakeRotator 0.0 0.0 (.Yaw (Math|Rotator|BreakRotator (Pawn|GetControlRotation :!class /Script/Engine.Pawn))))) AxisValue))

(event Input|AxisEvents|InputAxisMouseX
  (params (AxisValue :type Float%20%28single-precision%29))
  ;[1 1 1] Rotation
  (Pawn|Input|AddControllerYawInput AxisValue))

(event Input|AxisEvents|InputAxisMouseY
  (params (AxisValue :type Float%20%28single-precision%29))
  ;[1 1 1] Rotation
  (Pawn|Input|AddControllerPitchInput AxisValue))

(fn ConstructionScript)

(fn GetPawnForward
  (return (Math|Vector|GetForwardVector (Math|Rotator|MakeRotator 0.0 0.0 (.Yaw (Math|Rotator|BreakRotator (Pawn|GetControlRotation :!class /Script/Engine.Pawn)))))))