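; Player character for a 3D platformer, with buffered and coyote jumps, double jump, wall slide and jump, and an air-limited dash.
; Tick updates timer-driven movement states; wall sliding uses a forward trace and constrains input to the wall normal.
; Enemy hits cause damage, knockback and blinking invincibility; death respawns at the starting transform behind a screen transition.
; It also owns the health and coin HUD and pause menu.
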(event Custom|Death
  ;[1 1 1] Death
  (Utilities|Time|SetTimerbyFunctionName self "Respawn" (Variables|/Game/Blueprints/UI/RespawnTransition.RespawnTransition_C|GettransitionDuration (Variables|Default|GetrespawnTransition)))
  (Default|StartExitTranstion (Variables|Default|GetrespawnTransition)))

(event Custom|ResetDoubleJump
  ;[1 1 1] Double-Jumping
  ;;[1 1 1] Reset
  (if (and (AI|Components|NavMovement|IsMovingonGround (Variables|Character|GetCharacterMovement)) (Variables|Default|GethasDoubleJumped))
    (Variables|Default|SethasDoubleJumped false)))

(event Custom|WallSlide
  (bind _returnvalue (Transformation|GetActorLocation))
  (bind _charactermovement (Variables|Character|GetCharacterMovement))
  ;[1 1 1] Wall Sliding
  ;;[1 1 1] Reset
  (if (AI|Components|NavMovement|IsMovingonGround (Variables|Character|GetCharacterMovement))
    (if (Class|KismetMathLibrary|NotEqualExactlyVectorVector (Variables|Default|GetwallSlideNormal) "0, 0, 0")
      (Variables|Default|SetwallSlideNormal "0, 0, 0")
      (Variables|Default|SetisWallSliding false :!label _label))
    (elif (< (.Z (Math|Vector|BreakVector (Variables|/Script/Engine.MovementComponent|GetVelocity (Variables|Character|GetCharacterMovement)))) 0.0)
      ;;[1 1 1] Check if the player is against a wall
      (bind (_hit _hitnormal) (CallFunction|Raycast _returnvalue (+ _returnvalue (* (Transformation|GetActorForwardVector) 5e+01))))
      (if (and _hit (<= (Math|Vector|DotProduct _hitnormal "0,0.000000,1.000000") 0.01))
        (Utilities|FlowControl|Sequence
          (:then_0
            (if (not (Variables|Default|GetisWallSliding))
              (Animation|PlayAnimMontage "/Game/Assets/Characters/Neko/Montages/Montage_NekoWallSlide.Montage_NekoWallSlide" 1.0 "None") ; Start wall slide anim on first frame of wall slide.
            ))
          (:then_1
            (Variables|Default|SetisWallSliding true)
            (Variables|Default|SetwallSlideNormal _hitnormal)
            (Transformation|SetActorRotation (Math|Conversions|RotationFromXVector (Math|Vector|MakeVector (.X (Math|Vector|BreakVector (* _hitnormal -1.0))) (.Y (Math|Vector|BreakVector (* _hitnormal -1.0))) 0.0)))
            ;;[1 1 1] Slow down the fall
            (Variables|/Script/Engine.MovementComponent|SetVelocity _charactermovement (Math|Vector|MakeVector (.X (Math|Vector|BreakVector (* (Variables|Default|GetwallSlideNormal) (Math|Vector|DotProduct (Variables|/Script/Engine.MovementComponent|GetVelocity _charactermovement) (Variables|Default|GetwallSlideNormal))))) (.Y (Math|Vector|BreakVector (* (Variables|Default|GetwallSlideNormal) (Math|Vector|DotProduct (Variables|/Script/Engine.MovementComponent|GetVelocity _charactermovement) (Variables|Default|GetwallSlideNormal))))) (* -1 (Variables|Default|GetwallSlideSpeed))))))
        (else
          (Variables|Default|SetisWallSliding false)))
      (elif (Variables|Default|GetisWallSliding)
        (goto _label)))))

(event Custom|DoubleJump
  ;[1 1 1] Double-Jumping
  (if (Math|Boolean|ANDBoolean (AI|Components|NavMovement|IsFalling (Variables|Character|GetCharacterMovement)) (not (Variables|Default|GethasDoubleJumped)) (not (Variables|Default|GetisWallSliding)))
    (Variables|Default|SetjumpBuffer 0.0)
    (Character|LaunchCharacter (Math|Vector|MakeVector 0.0 0.0 (+ (* (.Z (Math|Vector|BreakVector (Variables|/Script/Engine.MovementComponent|GetVelocity (Variables|Character|GetCharacterMovement)))) -1.0) (Variables|Default|GetdoubleJumpZVelocity))) false false)
    (Animation|PlayAnimMontage "/Game/Assets/Characters/Neko/Montages/Montage_NekoJump.Montage_NekoJump" 1.0 "Default")
    (if (> (Variables|Default|GetkoyoteJumpBuffer) 0.0)
      (Variables|Default|SetkoyoteJumpBuffer 0.0)
      (else
        (Variables|Default|SethasDoubleJumped true)))))

(event Custom|WallJump
  ;[1 1 1] Wall Jump
  (if (Variables|Default|GetisWallSliding)
    (Character|LaunchCharacter (+ (* (* (Math|Vector|GetForwardVector (Transformation|GetActorRotation)) (Variables|Default|GetwallJumpXYVelocity)) -1.0) (Math|Vector|MakeVector 0.0 0.0 (Variables|Default|GetwallJumpZVelocity))) false false)
    (Transformation|SetActorRotation (Math|Conversions|RotationFromXVector (Variables|Default|GetwallSlideNormal)))
    (Variables|Default|SetisWallSliding false)
    (Animation|PlayAnimMontage "/Game/Assets/Characters/Neko/Montages/Montage_NekoJump.Montage_NekoJump" 1.0 "Default")))

(event Custom|MoveInDirection
  (params (Direction :type Vector) (Scale%20Value :type Float%20%28single-precision%29))
  (bind _wallslidenormal (Variables|Default|GetwallSlideNormal))
  ;[1 1 1] Movement
  (if (Variables|Default|GetisWallSliding)
    (Pawn|Input|AddMovementInput _wallslidenormal (* (Math|Vector|DotProduct _wallslidenormal Direction) Scale%20Value) false)
    (else
      (Pawn|Input|AddMovementInput Direction Scale%20Value false))))

(event Custom|Dash
  (bind _charactermovement (Variables|Character|GetCharacterMovement))
  ;[1 1 1] Dashing
  (if (Variables|Default|GetisDashing)
    (if (> (Variables|Default|GetdashTimer) 0.0)
      (Variables|Default|SetdashTimer (- (Variables|Default|GetdashTimer) (Utilities|Time|GetWorldDeltaSeconds)))
      (Transformation|SetActorLocation (+ (* (Math|Vector|GetForwardVector (Variables|Collision|GetCapsuleComponent)) (Variables|Default|GetdashVelocity)) (Transformation|GetActorLocation)) false false)
      (Variables|/Script/Engine.MovementComponent|SetVelocity _charactermovement (Math|Vector|MakeVector (.X (Math|Vector|BreakVector (Variables|/Script/Engine.MovementComponent|GetVelocity _charactermovement))) (.Y (Math|Vector|BreakVector (Variables|/Script/Engine.MovementComponent|GetVelocity _charactermovement))) 0.0))
      (else
        (Variables|Default|SetisDashing false)))
    (elif (AI|Components|NavMovement|IsMovingonGround (Variables|Character|GetCharacterMovement))
      (Variables|Default|SethasDashed false))))

(event Custom|Invincibility
  ;[1 1 1] Invincibility
  (if (> (Variables|Default|GetinvincibilityTimer) 0.0)
    (Variables|Default|SetinvincibilityTimer (- (Variables|Default|GetinvincibilityTimer) (Utilities|Time|GetWorldDeltaSeconds)))
    (if (<= (Variables|Default|GetinvincibilityTimer) 0.0)
      (CallFunction|ToggleBlinking false))))

(event Custom|JumpBuffering
  ;[1 1 1] Jump Buffering
  (if (> (Variables|Default|GetjumpBuffer) 0.0)
    (Variables|Default|SetjumpBuffer (- (Variables|Default|GetjumpBuffer) (Utilities|Time|GetWorldDeltaSeconds)))
    (if (AI|Components|NavMovement|IsMovingonGround (Variables|Character|GetCharacterMovement))
      (Character|Jump)
      (Variables|Default|SetjumpBuffer 0.0))))

(event Custom|KoyoteJump
  (bind _charactermovement (Variables|Character|GetCharacterMovement))
  (bind _returnvalue (AI|Components|NavMovement|IsFalling _charactermovement))
  ;[1 1 1] Koyote Jumping
  (Utilities|FlowControl|Sequence
    (:then_0
      (if (and _returnvalue (not (Variables|Default|GetwasFalling)))
        (Variables|Default|SetkoyoteJumpBuffer (Variables|Default|GetjumpBufferDuration))))
    (:then_1
      (Variables|Default|SetwasFalling _returnvalue))
    (:then_2
      (if (> (Variables|Default|GetkoyoteJumpBuffer) 0.0)
        (Variables|Default|SetkoyoteJumpBuffer (- (Variables|Default|GetkoyoteJumpBuffer) (Utilities|Time|GetWorldDeltaSeconds)))))))

(event EventOnLanded
  (params (Hit :type Hit%20Result%20Structure%20%28by%20ref%29))
  ;[1 1 1] Landing Animation
  (Animation|PlayAnimMontage "/Game/Assets/Characters/Neko/Montages/Montage_NekoJump.Montage_NekoJump" 3.0 "Land"))

(event EventTick
  (params (DeltaSeconds :type Float%20%28single-precision%29))
  ;[1 1 1] Tick Update
  (CallFunction|ResetDoubleJump)
  (CallFunction|JumpBuffering)
  (CallFunction|KoyoteJump)
  (CallFunction|WallSlide)
  (CallFunction|Dash)
  (CallFunction|Invincibility))

(event EventBeginPlay
  ;[1 1 1] Create the respawn transition and the HUD
  (bind _returnvalue (UserInterface|CreateWidget "/Game/Blueprints/UI/RespawnTransition.RespawnTransition_C"))
  (bind _output_get (Variables|Default|SetrespawnTransition _returnvalue))
  (UserInterface|Viewport|AddtoViewport _output_get 1)
  (Default|StartEnterTransition _output_get)
  (bind _returnvalue_2 (UserInterface|CreateWidget "/Game/Blueprints/UI/InGameHud.InGameHud_C"))
  (bind _output_get_2 (Variables|Default|SethealthHud _returnvalue_2))
  (UserInterface|Viewport|AddtoViewport _output_get_2 0)
  (Default|CreateHealth _output_get_2 (Variables|Default|GetmaxHealth))
  (bind _returnvalue_3 (Game|GetCurrentLevelName true))
  (if (Utilities|Enum|Equal(Enum) _returnvalue_3 "MainLevel")
    (Widget|SetVisibility (Variables|Default|GethealthHud) "Visible")
    (else
      (Widget|SetVisibility (Variables|Default|GethealthHud) "Hidden"))))

(event Collision|EventHit
  (params (MyComp :type Primitive%20Component%20Object%20Reference) (Other :type Actor%20Object%20Reference) (OtherComp :type Primitive%20Component%20Object%20Reference) (bSelfMoved :type Boolean) (HitLocation :type Vector :default "0, 0, 0") (HitNormal :type Vector :default "0, 0, 0") (NormalImpulse :type Vector :default "0, 0, 0") (Hit :type Hit%20Result%20Structure%20%28by%20ref%29))
  ;[1 1 1] Health
  (if (and (Utilities|Array|ContainsItem (Variables|/Script/Engine.Actor|GetTags Other) "Enemy") (<= (Variables|Default|GetinvincibilityTimer) 0.0))
    (CallFunction|InflictDamage 1 HitNormal)))

(event Input|ActionEvents|InputActionJump
  (params (Key :type Key%20Structure :default "None"))
  ;[1 1 1] Jumping
  (:Pressed
    (if (AI|Components|NavMovement|IsMovingonGround (Variables|Character|GetCharacterMovement))
      (Character|Jump)
      (Animation|PlayAnimMontage "/Game/Assets/Characters/Neko/Montages/Montage_NekoJump.Montage_NekoJump" 1.0 "Default")
      (else
        (Variables|Default|SetjumpBuffer (Variables|Default|GetjumpBufferDuration))
        (CallFunction|DoubleJump)
        (CallFunction|WallJump))))
  (:Released
    (Character|StopJumping)))

(event Input|ActionEvents|InputActionDash
  (params (Key :type Key%20Structure :default "None"))
  ;[1 1 1] Dashing
  (:Pressed
    (if (not (Variables|Default|GethasDashed))
      (Variables|Default|SetisDashing true)
      (Variables|Default|SethasDashed true)
      (Variables|Default|SetdashTimer (Variables|Default|GetdashDuration))
      (Animation|PlayAnimMontage "/Game/Assets/Characters/Neko/Montages/Montage_NekoDash.Montage_NekoDash" 1.0 "None"))))

(event Input|ActionEvents|InputActionPauseGame
  (params (Key :type Key%20Structure :default "None"))
  (bind _returnvalue (Game|GetPlayerController 0))
  ;[1 1 1] Pause/Unpause Game
  (:Pressed
    (Utilities|IsValid (Variables|Default|GetpauseMenu)
      (:Is%20Valid
        _)
      (:Is%20Not%20Valid
        (bind _returnvalue_2 (UserInterface|CreateWidget "/Game/Blueprints/UI/PauseScreen.PauseScreen_C"))
        (Variables|Default|SetpauseMenu _returnvalue_2)))
    (if (Game|IsGamePaused)
      (Widget|RemovefromParent (Variables|Default|GetpauseMenu))
      (Game|SetGamePaused false)
      (Variables|/Script/Engine.PlayerController|SetbShowMouseCursor _returnvalue false)
      (Input|SetInputModeGameOnly _returnvalue)
      (else
        (UserInterface|Viewport|AddtoViewport (Variables|Default|GetpauseMenu) 0)
        (Game|SetGamePaused true)
        (Variables|/Script/Engine.PlayerController|SetbShowMouseCursor _returnvalue true)
        (Input|SetInputModeGameandUI _returnvalue (Variables|Default|GetpauseMenu) "LockInFullscreen" false)))))

(event Input|AxisEvents|InputAxisLateralMovement
  (params (AxisValue :type Float%20%28single-precision%29))
  ;[1 1 1] Movement
  (CallFunction|MoveinDirection (Math|Vector|GetRightVector (Math|Rotator|MakeRotator 0.0 0.0 (.Yaw (Math|Rotator|BreakRotator (Pawn|GetControlRotation :!class /Script/Engine.Pawn))))) AxisValue))

(event Input|AxisEvents|InputAxisForwardMovement
  (params (AxisValue :type Float%20%28single-precision%29))
  ;[1 1 1] Movement
  (CallFunction|MoveinDirection (Math|Vector|GetForwardVector (Math|Rotator|MakeRotator 0.0 0.0 (.Yaw (Math|Rotator|BreakRotator (Pawn|GetControlRotation :!class /Script/Engine.Pawn))))) AxisValue))

(event Input|AxisEvents|InputAxisMouseX
  (params (AxisValue :type Float%20%28single-precision%29))
  ;[1 1 1] Rotation
  (Pawn|Input|AddControllerYawInput AxisValue))

(event Input|AxisEvents|InputAxisMouseY
  (params (AxisValue :type Float%20%28single-precision%29))
  ;[1 1 1] Rotation
  (Pawn|Input|AddControllerPitchInput AxisValue))

(fn ConstructionScript
  (Variables|Default|SetrespawnPos (Transformation|GetActorTransform)))

(fn GetPawnForward
  (return (Math|Vector|GetForwardVector (Math|Rotator|MakeRotator 0.0 0.0 (.Yaw (Math|Rotator|BreakRotator (Pawn|GetControlRotation :!class /Script/Engine.Pawn)))))))

(fn Respawn
  (bind _respawnpos (Variables|Default|GetrespawnPos))
  (bind (_location _rotation _scale) (Math|Transform|BreakTransform _respawnpos))
  (Transformation|SetActorTransform (Math|Transform|MakeTransform (+ (* (Variables|/Script/Engine.MovementComponent|GetVelocity (Variables|Character|GetCharacterMovement)) (* (Utilities|Time|GetWorldDeltaSeconds) -1.0)) _location) _rotation _scale))
  (Variables|/Script/Engine.MovementComponent|SetVelocity (Variables|Character|GetCharacterMovement) "0, 0, 0")
  (Variables|Default|SetinvincibilityTimer 0.0)
  (CallFunction|ToggleBlinking false)
  (Variables|Default|Sethealth 5)
  (Default|UpdateHealth (Variables|Default|GethealthHud) (Variables|Default|GetmaxHealth) (Variables|Default|Gethealth))
  (Default|StartEnterTransition (Variables|Default|GetrespawnTransition)))

(fn InflictDamage
  (params (amount :type Integer) (hitNormal :type Vector))
  (bind (_x _y) (Math|Vector|BreakVector hitNormal))
  ;[1 1 1] Decrease Health
  (Variables|Default|Sethealth (Math|Integer|Clamp(Integer) (- (Variables|Default|Gethealth) amount) 0 (Variables|Default|GetmaxHealth)))
  ;[1 1 1] Update Ui
  (Default|UpdateHealth (Variables|Default|GethealthHud) (Variables|Default|GetmaxHealth) (Variables|Default|Gethealth))
  (Utilities|FlowControl|Sequence
    (:then_0
      ;[1 1 1] Check if the player is dead
      (if (<= (Variables|Default|Gethealth) 0)
        (CallFunction|Death)))
    (:then_1
      ;[1 1 1] Start invincibility
      (if (> amount 0)
        (Variables|Default|SetinvincibilityTimer (Variables|Default|GetinvincibilityDuration))
        (CallFunction|ToggleBlinking true)
        ;[1 1 1] Knockback
        (if (and (!= (Variables|Default|Gethealth) 0) (Math|Vector|NotEqual(Vector) hitNormal "0, 0, 0" 0.0001))
          (Character|LaunchCharacter (* (Math|Vector|MakeVector _x _y 0.5) (Variables|Default|GetdamageKnockbackStrength)) false false))))))

(fn AddCoins
  (params (amount :type Integer))
  (Variables|Default|Setcoins (+ amount (Variables|Default|Getcoins)))
  (Default|UpdateCoins (Variables|Default|GethealthHud) (Variables|Default|Getcoins)))

(fn Raycast
  (params (Start :type Vector) (End :type Vector))
  (bind (_outhit _returnvalue) (Collision|LineTraceByChannel Start End "TraceTypeQuery1" false 0 "None"))
  (return _returnvalue (.ImpactNormal (Collision|BreakHitResult _outhit))))

(fn ToggleBlinking
  (params (blink :type Boolean))
  (bind _mesh (Variables|Character|GetMesh))
  (if blink
    (Rendering|Material|SetMaterial _mesh 0 "/Game/Assets/Materials/GradientBlinking.GradientBlinking")
    (Rendering|Material|SetMaterial _mesh 1 "/Game/Assets/Characters/Neko/Materials/NekoMouthBlinking.NekoMouthBlinking")
    (else
      (Rendering|Material|SetMaterial _mesh 0 "/Game/Assets/Materials/Gradient.Gradient")
      (Rendering|Material|SetMaterial _mesh 1 "/Game/Assets/Characters/Neko/Materials/NekoMouth.NekoMouth"))))

(fn ToggleHud
  (bind _healthhud (Variables|Default|GethealthHud))
  (if (Utilities|Enum|Equal(Enum) (Widget|GetVisibility (Variables|Default|GethealthHud)) "Visible")
    (Widget|SetVisibility _healthhud "Hidden")
    (else
      (Widget|SetVisibility _healthhud "Visible"))))