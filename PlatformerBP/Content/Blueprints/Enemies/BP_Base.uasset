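; Base enemy character that a PlatformerPlayer damages by stomping on it.
; Bump checks that the player is falling, calls ReceiveDamage and launches the player back up with reversed fall speed plus a boost.
; ReceiveDamage decrements health; at zero the enemy is destroyed, with a one-in-five chance to spawn a HealthCollectible.
; The event graph also holds player-style input handlers for look, wall-slide-aware movement and walk-speed toggling.
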(event Custom|Death
  (Actor|DestroyActor))

(event Input|ActionEvents|InputActionWalk
  (params (Key :type Key%20Structure))
  (bind _charactermovement (Variables|Character|GetCharacterMovement))
  ;[1 1 1] Walk
  (:Pressed
    (bind _output_get (Variables|Default|SetWalkTemp (not (Variables|Default|GetWalkTemp))))
    (if _output_get
      (Variables|/Script/Engine.CharacterMovementComponent|SetMaxWalkSpeed _charactermovement 6e+02)
      (else
        (Variables|/Script/Engine.CharacterMovementComponent|SetMaxWalkSpeed _charactermovement 3e+02)))))

(event Input|AxisEvents|InputAxisLateralMovement
  (params (AxisValue :type Float%20%28single-precision%29))
  (bind _returnvalue (Pawn|GetControlRotation :!class /Script/Engine.Pawn))
  (bind _wallslidenormal (Variables|Default|GetwallSlideNormal))
  (bind _yaw (Math|Rotator|BreakRotator _returnvalue))
  (bind _returnvalue_2 (Math|Rotator|MakeRotator 0.0 0.0 _yaw))
  (bind _returnvalue_3 (Math|Vector|GetRightVector _returnvalue_2))
  ;[1 1 1] Movement
  (if (Variables|Default|GetisWallSliding)
    (Pawn|Input|AddMovementInput _wallslidenormal (* AxisValue (Math|Vector|DotProduct _wallslidenormal _returnvalue_3)) false)
    (else
      (Pawn|Input|AddMovementInput _returnvalue_3 AxisValue false))))

(event Input|AxisEvents|InputAxisForwardMovement
  (params (AxisValue :type Float%20%28single-precision%29))
  (bind _returnvalue (Pawn|GetControlRotation :!class /Script/Engine.Pawn))
  (bind _wallslidenormal (Variables|Default|GetwallSlideNormal))
  (bind _yaw (Math|Rotator|BreakRotator _returnvalue))
  (bind _returnvalue_2 (Math|Rotator|MakeRotator 0.0 0.0 _yaw))
  (bind _returnvalue_3 (Math|Vector|GetForwardVector _returnvalue_2))
  ;[1 1 1] Movement
  (if (Variables|Default|GetisWallSliding)
    (Pawn|Input|AddMovementInput _wallslidenormal (* AxisValue (Math|Vector|DotProduct _wallslidenormal _returnvalue_3)) false)
    (else
      (Pawn|Input|AddMovementInput _returnvalue_3 AxisValue false))))

(event Input|AxisEvents|InputAxisMouseX
  (params (AxisValue :type Float%20%28single-precision%29))
  ;[1 1 1] Rotation
  (Pawn|Input|AddControllerYawInput AxisValue))

(event Input|AxisEvents|InputAxisMouseY
  (params (AxisValue :type Float%20%28single-precision%29))
  ;[1 1 1] Rotation
  (Pawn|Input|AddControllerPitchInput AxisValue))

(fn ConstructionScript)

(fn ReceiveDamage
  ;[1 1 1] Damage Enemies
  (Variables|Default|Sethealth (Math|Integer|Clamp(Integer) (- (Variables|Default|Gethealth) 1) 0 (Variables|Default|GetmaxHealth)))
  (if (<= (Variables|Default|Gethealth) 0)
    (CallFunction|Death)
    (if (== (Math|Random|RandomIntegerinRange 0 4) 0)
      (Game|SpawnActorfromClass "/Game/Blueprints/Collectibles/HealthCollectible.HealthCollectible_C" (Transformation|GetActorTransform) "Undefined" 0 0))))

(fn Bump
  (params (Object :type Actor%20Object%20Reference))
  ;[1 1 1] Bump
  (bind _asplatformer_player (Utilities|Casting|CastToPlatformerPlayer Object))
  (if (< (.Z (Math|Vector|BreakVector (Variables|/Script/Engine.MovementComponent|GetVelocity (Variables|/Script/Engine.Character|GetCharacterMovement _asplatformer_player)))) 0.0)
    (CallFunction|ReceiveDamage)
    (Character|LaunchCharacter _asplatformer_player (+ (* (Math|Vector|MakeVector 0.0 0.0 (.Z (Math|Vector|BreakVector (Variables|/Script/Engine.MovementComponent|GetVelocity (Variables|/Script/Engine.Character|GetCharacterMovement _asplatformer_player))))) -1.0) (Math|Vector|MakeVector 0.0 0.0 5e+02)) false false)))