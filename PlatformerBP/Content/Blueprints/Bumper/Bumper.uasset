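; Bumper is a bouncy mushroom actor that launches a falling PlatformerPlayer along its own up vector when overlapped.
; The additive launch negates the player's current velocity and adds BumpSpeed along that vector, so incoming momentum is cancelled and rotation sets the bounce direction.
; Each bounce resets the double jump, plays the shroom animation, and plays a jump montage on the tagged player cached at BeginPlay.
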(event EventBeginPlay
  (bind _outactors (Actor|GetAllActorsOfClasswithTag "/Game/Blueprints/Player/PlatformerPlayer.PlatformerPlayer_C" "Player"))
  (Variables|Default|SetplayerRef (Utilities|Array|Get(acopy) _outactors)))

(event Collision|EventActorBeginOverlap
  (params (OtherActor :type Actor%20Object%20Reference))
  (bind _asplatformer_player (Utilities|Casting|CastToPlatformerPlayer OtherActor))
  (if (< (.Z (Math|Vector|BreakVector (Variables|/Script/Engine.MovementComponent|GetVelocity (Variables|/Script/Engine.Character|GetCharacterMovement _asplatformer_player)))) 0.0)
    (Character|LaunchCharacter _asplatformer_player (+ (Math|Vector|NegateVector (Variables|/Script/Engine.MovementComponent|GetVelocity (Variables|/Script/Engine.Character|GetCharacterMovement _asplatformer_player))) (* (Transformation|GetActorUpVector) (Variables|Default|GetbumpSpeed))) false false)
    (Variables|/Game/Blueprints/Player/PlatformerPlayer.PlatformerPlayer_C|SethasDoubleJumped _asplatformer_player false)
    (Components|Animation|PlayAnimation (Variables|Default|GetBumpShroom) "/Game/Assets/Plants/BumpShroom/BumpShroom_Anim.BumpShroom_Anim" false)
    (Animation|PlayAnimMontage (Variables|Default|GetplayerRef) "/Game/Assets/Characters/Neko/Montages/Montage_NekoJump.Montage_NekoJump" 1.0 "Default")))

(fn ConstructionScript)