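; Checkpoint actor that sets the player's respawn point the first time the player touches it.
; On actor overlap, it casts the other actor to PlatformerPlayer and copies its own transform into that player's RespawnPos.
; A WasActivated flag makes it one-shot, and activation hides the FlagWhite component and shows Flag as visual feedback.
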(event Collision|EventActorBeginOverlap
  (params (OtherActor :type Actor%20Object%20Reference))
  (if (not (Variables|Default|GetwasActivated))
    (bind _asplatformer_player (Utilities|Casting|CastToPlatformerPlayer OtherActor))
    (Variables|/Game/Blueprints/Player/PlatformerPlayer.PlatformerPlayer_C|SetrespawnPos _asplatformer_player (Transformation|GetActorTransform))
    (Variables|Default|SetwasActivated true)
    (Rendering|SetVisibility (Variables|Default|GetFlagWhite) false false)
    (Rendering|SetVisibility (Variables|Default|GetFlag) true false)))

(fn ConstructionScript)